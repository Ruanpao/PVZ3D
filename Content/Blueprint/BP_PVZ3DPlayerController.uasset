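; Player controller for a 3D PVZ game that owns the on-screen minimap.
; On BeginPlay it creates the minimap widget with a background texture, the controlled pawn and a fixed map size, stores it and adds it to the viewport.
; Pressing Tab toggles the stored widget between visible and hidden.
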(event EventBeginPlay
  (bind _returnvalue (UserInterface|CreateWidget "/Game/UI/WBP_MiniMap.WBP_MiniMap_C" 0 "/Game/MyAsset/MiniMap/T_MiniMapBackImage.T_MiniMapBackImage" 0.2 (Pawn|GetControlledPawn) "(X=30600.000000,Y=13200.000000)"))
  (bind _output_get (Variables|Default|SetMiniMapUI _returnvalue))
  (UserInterface|Viewport|AddtoViewport (Variables|Default|GetMiniMapUI) 0))

(event Input|KeyboardEvents|Tab
  (params (Key :type Key%20Structure :default "None"))
  (bind _minimapui (Variables|Default|GetMiniMapUI))
  (:Pressed
    (Utilities|IsValid _minimapui
      (:Is%20Valid
        (if (Widget|IsVisible _minimapui)
          (Widget|SetVisibility _minimapui "Hidden")
          (else
            (Widget|SetVisibility _minimapui "Visible")))))))

(fn ConstructionScript)